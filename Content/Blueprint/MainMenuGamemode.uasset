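; Main menu game mode for a tanks game that shows the menu and launches a match with the joined players.
; BeginPlay creates the main menu and a join-players popup, binding their events; Play shows the popup, while Settings creates a settings widget on each press.
; Confirming the popup stores four player states in TanksGameInstance to carry them into GameLevel, adding P4 before P3.
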(event `self.ReceiveBeginPlay`
  (bind _returnvalue (`|CreateWidget` (`self.MainMenuWidget`)))
  (`UserWidget.AddToViewport` _returnvalue 0)
  (bind _asmain_menu_widget (cast `/Game/Blueprint/MainMenuWidget` _returnvalue))
  (add `/Game/Blueprint/MainMenuWidget.PlayGameHit` _asmain_menu_widget (delegate `Play Hit`))
  (add `/Game/Blueprint/MainMenuWidget.SettingsHit` _asmain_menu_widget (delegate `Settings Hit`))
  (bind _returnvalue_2 (`|CreateWidget` (`self.JoinPlayersWidget`)))
  (bind _asjoin_players_widget (cast `/Game/Blueprint/JoinPlayersWidget` _returnvalue_2))
  (add `/Game/Blueprint/JoinPlayersWidget.PlayHit` _asjoin_players_widget (delegate `PopupPlayHit`)))

(event `Play Hit`
  (`UserWidget.AddToViewport` (stale `self.ReceiveBeginPlay` _returnvalue_2) 0))

(event `Settings Hit`
  ;[1 1 1] Show settings widget
  (bind _returnvalue (`|CreateWidget` (`self.SettingsWidget`)))
  (`UserWidget.AddToViewport` _returnvalue 0))

(event `PopupPlayHit`
  (params (P1State :type Integer) (P2State :type Integer) (P3State :type Integer) (P4State :type Integer))
  ;[1 1 1] Use the GameInstance to pass the menu settings between levels
  (bind _astanks_game_instance (cast `TanksGameInstance` (`GameplayStatics.GetGameInstance`)))
  (bind _joinedplayerstatus (`TanksGameInstance.joinedPlayerStatus` _astanks_game_instance))
  (`KismetArrayLibrary.Array_Clear` _joinedplayerstatus)
  (`KismetArrayLibrary.Array_Add` _joinedplayerstatus P1State)
  (`KismetArrayLibrary.Array_Add` _joinedplayerstatus P2State)
  (`KismetArrayLibrary.Array_Add` _joinedplayerstatus P4State)
  (`KismetArrayLibrary.Array_Add` _joinedplayerstatus P3State)
  (`GameplayStatics.OpenLevel` "GameLevel"))

(fn `UserConstructionScript`)