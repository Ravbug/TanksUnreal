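; Bullet_BP is a projectile actor that detects tank hits and destroys itself on impact.
; Its construction script feeds InitialVelocity into the ProjectileMovement component and sets a short lifespan.
; A counter skips the sphere's first overlap; any later overlap destroys the bullet, first printing a debug message if the other actor is a Tank_BP, without applying damage.
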(event `self.Sphere.OnComponentBeginOverlap`
  (params (OverlappedComponent :type "PrimitiveComponent Object Reference") (OtherActor :type "Actor Object Reference") (OtherComp :type "PrimitiveComponent Object Reference") (OtherBodyIndex :type Integer) (bFromSweep :type Boolean) (SweepResult :type "HitResult Structure (by ref)"))
  ;[1 1 1] On 2nd overlap, determine if hit a tank
  (bind _output_get (set `self.OverlapCount` (+ (`self.OverlapCount`) 1)))
  (if (> _output_get 1)
    (cast `/Game/Blueprint/Tank_BP` OtherActor
      (:`then`
        (`KismetSystemLibrary.PrintString` "Hit Tank"))
      (:`CastFailed`
        _))
    (`self.K2_DestroyActor`)))

(fn `UserConstructionScript`
  ;[1 1 1] Set initial velocity
  (set `ProjectileMovementComponent.InitialSpeed` (`self.InitialVelocity`) (`self.ProjectileMovement`))
  (`self.SetLifeSpan` 5.0))