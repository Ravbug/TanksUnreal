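; Tank Blueprint that handles the visual and spawning side of a tank, with a charge-shot bar, a health HUD and bullet firing.
; BeginPlay casts and caches both widget component objects to avoid repeated casts.
; Events, at least the charge bar one driven from C++, set the bar percentages or spawn Bullet_BP at the spawn point, passing the given amount as initial velocity.
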(event `self.ReceiveBeginPlay`
  ;[1 1 1] Initialize temporary variables to avoid unecessary casting
  (bind _asprogress_bar (cast `/Game/Blueprint/ProgressBar` (`WidgetComponent.GetUserWidgetObject` (`self.ChargeShotBar`))))
  (set `self.ChargeShotCasted` _asprogress_bar)
  (bind _astank_info_hud (cast `/Game/Blueprint/TankInfoHUD` (`WidgetComponent.GetUserWidgetObject` (`self.HealthInfoHUD`))))
  (set `self.Health HUD` _astank_info_hud))

(event `self.SetChargeBar`
  (params (amount :type "Float (single-precision)"))
  ;[1 1 1] Invoked when C++ sets the box amount
  (`ProgressBar.SetPercent` (`/Game/Blueprint/ProgressBar.Bar` (`self.ChargeShotCasted`)) amount))

(event `self.SapwnBullet`
  (params (amount :type "Float (single-precision)"))
  (`|SpawnActorFromClass` "/Game/Blueprint/Bullet_BP.Bullet_BP_C" (`SceneComponent.K2_GetComponentToWorld` (`self.BulletSpawnpoint`)) "Undefined" "OverrideRootScale" null amount null))

(event `self.SetHealthBar`
  (params (amount :type "Float (single-precision)"))
  (`ProgressBar.SetPercent` (`/Game/Blueprint/TankInfoHUD.HealthBar` (`self.Health HUD`)) amount))

(fn `UserConstructionScript`)