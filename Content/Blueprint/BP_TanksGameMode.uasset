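; Game mode Blueprint for a tanks game that manages the round-starting HUD.
; On BeginPlay it creates the level-starting widget for player 0 and caches it as a RoundNumHUD.
; DisplayRoundStarting sets the widget's label to the passed string and adds it to the viewport.
; ClearViewport removes that same widget, so one instance is reused rather than recreated.
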(event `self.ReceiveBeginPlay`
  ;[1 1 1] Initialize Widgets for HUD
  (bind _returnvalue (`|CreateWidget` (`self.LevelStartingWidget`) (`GameplayStatics.GetPlayerControllerFromID` 0)))
  (bind _asround_num_hud (cast `/Game/Blueprint/RoundNumHUD` _returnvalue))
  (set `self.Level Starting Widget` _asround_num_hud))

(event `self.DisplayRoundStarting`
  (params (str :type String))
  (bind _level_starting_widget (`self.Level Starting Widget`))
  ;[1 1 1] Display level starting HUD
  (`RichTextBlock.SetText` (`/Game/Blueprint/RoundNumHUD.Label` _level_starting_widget) (`KismetTextLibrary.Conv_StringToText` str))
  (`UserWidget.AddToViewport` _level_starting_widget 0))

(event `self.ClearViewport`
  (`Widget.RemoveFromParent` (`self.Level Starting Widget`)))

(fn `UserConstructionScript`)